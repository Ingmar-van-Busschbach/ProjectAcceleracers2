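; Player controller for driving that sets up the driver's input, speedometer HUD and pause menu.
; On BeginPlay it adds the Enhanced Input mapping context selected in GI_GlobalGameInstance, then creates that instance's selected speedometer widget, bound to the possessed BP_CarBase.
; The speedometer is skipped if the pawn is not a BP_CarBase at that moment.
; IA_Menu opens WBP_PauseMenu with UI-only input and a visible cursor, without pausing the game here.
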(event `self.ReceiveBeginPlay`
  (`|ExecutionSequence`
    (:`then_0`
      (`self.SetupInputMapping`))
    (:`then_1`
      (`self.SpawnSpeedometerUI`))))

(event `SpawnSpeedometerUI`
  (bind _asgi_global_game_instance (cast `/Game/Core/GI_GlobalGameInstance` (`GameplayStatics.GetGameInstance`)))
  (bind _asbp_car_base (cast `/Game/Core/Vehicles/BP_CarBase` (`self.K2_GetPawn`)))
  (bind _returnvalue (`|CreateWidget` (`/Game/Core/GI_GlobalGameInstance.SelectedSpeedometer` _asgi_global_game_instance) self _asbp_car_base))
  (`UserWidget.AddToViewport` _returnvalue 0))

(event `SetupInputMapping`
  (bind _asgi_global_game_instance (cast `/Game/Core/GI_GlobalGameInstance` (`GameplayStatics.GetGameInstance`)))
  (bind _selectedinputmappingcontext (`/Game/Core/GI_GlobalGameInstance.SelectedInputMappingContext` _asgi_global_game_instance))
  (`EnhancedInputSubsystemInterface.AddMappingContext` (subsystem `EnhancedInputLocalPlayerSubsystem`) _selectedinputmappingcontext 0 (struct))
  (`/Game/Core/Engine/BPFL_DebugFunctions.PrintMessage` (`KismetSystemLibrary.GetObjectName` _selectedinputmappingcontext)))

(event `EnhancedInput|/Game/Core/Inputs/IA_Menu`
  (params (ActionValue :type Boolean) (ElapsedSeconds :type "Float (double-precision)") (TriggeredSeconds :type "Float (double-precision)") (InputAction :type "InputAction Object Reference" :default "/Game/Core/Inputs/IA_Menu.IA_Menu"))
  (:`Triggered`
    (bind _returnvalue (`|CreateWidget` "/Game/UI/IngameMenu/WBP_PauseMenu.WBP_PauseMenu_C"))
    (`UserWidget.AddToViewport` _returnvalue 0)
    (`WidgetBlueprintLibrary.SetInputMode_UIOnlyEx` self _returnvalue "DoNotLock" true)
    (set `self.bShowMouseCursor` true)))

(fn `UserConstructionScript`)