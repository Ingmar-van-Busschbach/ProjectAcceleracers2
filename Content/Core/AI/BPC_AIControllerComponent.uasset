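; AI driver component that takes over its owning BP_CarBase, disabling player input and manual shifting to follow a spline.
; Each tick samples look-ahead points along SplineRef, blending direction-to-point and spline-heading yaw errors through AISettings curves.
; Corner-based target speed versus current speed drives throttle, weighted toward far samples; steering favours near samples.
; A sphere trace runs at each sample, but its hits are unused.
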(event `self.ReceiveBeginPlay`
  (bind _asbp_car_base (cast `/Game/Core/Vehicles/BP_CarBase` (`self.GetOwner`)))
  (bind _output_get (set `self.PawnRef` _asbp_car_base))
  (set `/Game/Core/Vehicles/BP_CarBase.TickReadPlayerInput` false _output_get)
  (set `/Game/Core/Vehicles/BP_EngineComponent.ManualGearShifting` false (`/Game/Core/Vehicles/BP_CarBase.BP_EngineComponent` _output_get)))

(event `self.ReceiveTick`
  (params (DeltaSeconds :type "Float (single-precision)"))
  (bind _pawnref (`self.PawnRef`))
  (bind _pawnref_2 (`self.PawnRef`))
  (bind _aisettings (`self.AISettings`))
  (bind _splineref (`self.SplineRef`))
  (bind _aisettings_2 (`self.AISettings`))
  (bind _aisettings_3 (`self.AISettings`))
  (bind _pawnref_3 (`self.PawnRef`))
  (bind _returnvalue (`Actor.K2_GetActorLocation` (`self.PawnRef`)))
  (bind _returnvalue_2 (`Actor.K2_GetActorRotation` _pawnref_3))
  (bind _iterations (`/Game/Core/AI/PDA_AISettings.Iterations` (`self.AISettings`)))
  (bind _iterations_2 (`/Game/Core/AI/PDA_AISettings.Iterations` (`self.AISettings`)))
  (bind _iterations_3 (`/Game/Core/AI/PDA_AISettings.Iterations` (`self.AISettings`)))
  (`/Engine/EditorBlueprintResources/StandardMacros.IsValid` (`self.SplineRef`)
    (:`Is Valid`
      (`/Engine/EditorBlueprintResources/StandardMacros.IsValid` _pawnref_2
        (:`Is Valid`
          (set `/Game/Core/Vehicles/BP_CarBase.ThrottleInput` 0.0 _pawnref_2)
          (set `/Game/Core/Vehicles/BP_CarBase.SteeringInput` 0.0 _pawnref_2)
          (for _index (range (+ _iterations 1))
            (set `self.CurrentIteration` _index)
            (bind _returnvalue_3 (+ (`KismetMathLibrary.Lerp` (`/Game/Core/AI/PDA_AISettings.MinSimulationDistance` _aisettings) (`/Game/Core/AI/PDA_AISettings.MaxSimulationDistance` _aisettings) (* (/ (+ 0.5 0.5) _iterations) _index)) (`SplineComponent.GetDistanceAlongSplineAtLocation` _splineref _returnvalue "World")))
            (bind _returnvalue_4 (`SplineComponent.GetLocationAtDistanceAlongSpline` _splineref _returnvalue_3 "World"))
            (bind _yaw (.yaw (`KismetMathLibrary.NormalizedDeltaRotator` (`KismetMathLibrary.MakeRotFromXZ` (- _returnvalue_4 _returnvalue) (`Actor.GetActorUpVector` _pawnref_3)) _returnvalue_2)))
            (bind _yaw_2 (.yaw (`KismetMathLibrary.NormalizedDeltaRotator` _returnvalue_2 (`SplineComponent.GetRotationAtDistanceAlongSpline` _splineref _returnvalue_3 "World"))))
            (set `/Game/Core/Vehicles/BP_CarBase.ThrottleInput` (+ (`/Game/Core/Vehicles/BP_CarBase.ThrottleInput` _pawnref) (* (/ (`KismetMathLibrary.SelectFloat` 1.0 -1.0 (> (* (`self.MaxSpeedMultiplier`) (`CurveFloat.GetFloatValue` (`/Game/Core/AI/PDA_AISettings.ThrottleResponseCurve` (`self.AISettings`)) (`KismetMathLibrary.Lerp` (`CurveFloat.GetFloatValue` (`/Game/Core/AI/PDA_AISettings.CornerIntensityMap` _aisettings_3) _yaw) (`CurveFloat.GetFloatValue` (`/Game/Core/AI/PDA_AISettings.CornerIntensityMap` _aisettings_2) _yaw_2) 0.75))) (`/Game/Core/Vehicles/BP_EngineComponent.CurrentSpeed` (`/Game/Core/Vehicles/BP_CarBase.BP_EngineComponent` (`self.PawnRef`))))) _iterations_3) (/ (* (`self.CurrentIteration`) 2) _iterations_3))) _pawnref)
            (set `/Game/Core/Vehicles/BP_CarBase.SteeringInput` (+ (`/Game/Core/Vehicles/BP_CarBase.SteeringInput` _pawnref) (* (/ (`KismetMathLibrary.Lerp` (* (`CurveFloat.GetFloatValue` (`/Game/Core/AI/PDA_AISettings.SteeringResponseCurve` _aisettings_3) (`KismetMathLibrary.Abs` _yaw)) (`KismetMathLibrary.SignOfFloat` _yaw)) (* (`CurveFloat.GetFloatValue` (`/Game/Core/AI/PDA_AISettings.SteeringResponseCurve` _aisettings_2) (`KismetMathLibrary.Abs` _yaw_2)) (`KismetMathLibrary.SignOfFloat` _yaw_2) -1.0) 0.25) _iterations_2) (/ (- (* _iterations_2 2) (* (`self.CurrentIteration`) 2)) _iterations_2))) _pawnref)
            (`KismetSystemLibrary.SphereTraceMulti` :`Start` _returnvalue_4 :`End` _returnvalue_4 :`Radius` 200.0 :`TraceChannel` "TraceTypeQuery1" :`DrawDebugType` (select `bool` (`/Game/Core/Engine/BPFL_GlobalConstants.GlobalDebug`) :`true` "ForOneFrame" :!type "EDrawDebugTrace Enum"))))))))