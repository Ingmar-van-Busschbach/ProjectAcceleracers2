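; BP_AISpawner places an AI-driven car in the level at the spawner's location and rotation.
; On BeginPlay it spawns the Car pawn and adds a BPC AI controller component configured with its AISettings.
; It then gives that component a spline to reference from Track, falling back to Track0 when Track is not valid.
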(event `self.ReceiveBeginPlay`
  (bind _track (`self.Track`))
  (bind _track_0 (`self.Track_0`))
  (bind _returnvalue (`AIBlueprintHelperLibrary.SpawnAIFromClass` (`self.Car`) null (`self.K2_GetActorLocation`) (`self.K2_GetActorRotation`) false null))
  (bind _returnvalue_2 (`AddComponent|NODE_AddBPC_AIControllerComponent-0` :`self` _returnvalue :`RelativeTransform` (`KismetMathLibrary.MakeTransform` (0.0 0.0 0.0)) :`AISettings` (`self.AISettings`)))
  (`/Engine/EditorBlueprintResources/StandardMacros.IsValid` _track
    (:`Is Valid`
      (set `/Game/Core/AI/BPC_AIControllerComponent.SplineRef` (`/Game/Core/Objects/BP_SplineRoadTool.Spline` _track) _returnvalue_2))
    (:`Is Not Valid`
      (`/Engine/EditorBlueprintResources/StandardMacros.IsValid` _track_0
        (:`Is Valid`
          (set `/Game/Core/AI/BPC_AIControllerComponent.SplineRef` (`/Game/Core/Objects/SplineToolPro/Spline/SplineToolPro.Spline` _track_0) _returnvalue_2))))))

(fn `UserConstructionScript`)