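; BP_SplineRoadTool is an editor road-building tool that lays spline mesh segments along a spline in its construction script.
; It resizes the RoadSegments array to match, then creates each visible segment's mesh with position, tangents, scale and roll from the spline.
; FixedRoadLength switches between mesh-length steps and point-to-point segments.
; SplineOnlyMode skips rebuilds unless UpdateSpline is toggled, while EditMode skips material overrides, attachment and immediate mesh updates.
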(fn `UserConstructionScript`
  (bind _length (`self.GetMeshLength`))
  (bind _spline (`self.Spline`))
  (bind _index (`self.Index`))
  (bind _roadsegments (`self.RoadSegments`))
  (bind _spline_2 (`self.Spline`))
  (bind _spline_3 (`self.Spline`))
  (bind _spline_4 (`self.Spline`))
  (bind _meshlength (`self.MeshLength`))
  (bind _spline_5 (`self.Spline`))
  (bind _spline_6 (`self.Spline`))
  (bind _returnvalue (not (`self.EditMode`)))
  (bind _returnvalue_2 (not (`self.EditMode`)))
  (bind _returnvalue_3 (`SplineComponent.GetSplineLength` _spline_6))
  (bind _returnvalue_4 (`SplineComponent.GetSplineLength` _spline))
  (bind _returnvalue_5 (* (`self.Index`) _meshlength))
  (bind _returnvalue_6 (- (`self.NumberOfSplinePoints`) 1))
  (bind (_location _tangent) (`SplineComponent.GetLocationAndTangentAtSplinePoint` _spline_5 _index "Local"))
  (bind (_returnvalue_x _returnvalue_y _returnvalue_z) (`KismetMathLibrary.BreakVector` (`SplineComponent.GetScaleAtSplinePoint` (`self.Spline`) (`self.Index`))))
  (bind _returnvalue_7 (* (+ (`self.Index`) 1) (`self.MeshLength`)))
  (bind (_returnvalue_x_2 _returnvalue_y_2 _returnvalue_z_2) (`KismetMathLibrary.BreakVector` (`SplineComponent.GetScaleAtDistanceAlongSpline` (`self.Spline`) (* (`self.Index`) (`self.MeshLength`)))))
  (bind _returnvalue_8 (* (+ (`self.Index`) 1) (`self.MeshLength`)))
  (bind _returnvalue_9 (`SplineComponent.GetLocationAtDistanceAlongSpline` _spline_2 _returnvalue_5 "Local"))
  (bind _returnvalue_10 (`SplineComponent.GetDirectionAtDistanceAlongSpline` _spline_2 _returnvalue_5 "Local"))
  (bind (_location_2 _tangent_2) (`SplineComponent.GetLocationAndTangentAtSplinePoint` _spline_5 (- (`self.NumberOfSplinePoints`) 1) "Local"))
  (bind (_location_3 _tangent_3) (`SplineComponent.GetLocationAndTangentAtSplinePoint` _spline_5 (+ _index 1) "Local"))
  (bind (_returnvalue_x_3 _returnvalue_y_3 _returnvalue_z_3) (`KismetMathLibrary.BreakVector` (`SplineComponent.GetScaleAtSplinePoint` (`self.Spline`) (+ (`self.Index`) 1))))
  (bind _returnvalue_11 (+ _returnvalue_5 _meshlength))
  (bind (_returnvalue_x_4 _returnvalue_y_4 _returnvalue_z_4) (`KismetMathLibrary.BreakVector` (`SplineComponent.GetScaleAtDistanceAlongSpline` _spline_6 (`KismetMathLibrary.SelectFloat` _returnvalue_8 _returnvalue_3 (<= _returnvalue_8 _returnvalue_3)))))
  (if (`self.UpdateSpline`)
    (set `self.UpdateSpline` false)
    (set `self.MeshLength` _length :!label _label)
    (set `self.TangentLength` (`KismetMathLibrary.FClamp` (`self.TangentLength`) 0.0 _length))
    (set `self.EndTangentLength` (`KismetMathLibrary.FClamp` (`self.EndTangentLength`) 0.0 _length))
    (`|ExecutionSequence`
      (:`then_0`
        (`|ExecutionSequence`
          (:`then_0`
            (set `self.NumberOfSplinePoints` (`SplineComponent.GetNumberOfSplinePoints` (`self.Spline`))))
          (:`then_1`
            (set `self.NumberOfRoadSegments` (`.ReturnValue` (`KismetMathLibrary.FMod` (`SplineComponent.GetSplineLength` (`self.Spline`)) (`self.MeshLength`)))))
          (:`then_2`
            (`/Engine/EditorBlueprintResources/StandardMacros.CompareInt` (`KismetMathLibrary.SelectInt` (`self.NumberOfRoadSegments`) (`self.NumberOfSplinePoints`) (`self.FixedRoadLength`)) (`KismetArrayLibrary.Array_Length` (`self.RoadSegments`)) :!label _label_2
              (:`>`
                (`KismetArrayLibrary.Array_Add` (`self.RoadSegments`) (`self.RoadSettings`))
                (goto _label_2))
              (:`<`
                (`KismetArrayLibrary.Array_Remove` _roadsegments (`KismetArrayLibrary.Array_LastIndex` _roadsegments))
                (goto _label_2))))))
      (:`then_1`
        (if (`self.EditMode`)
          (`KismetArrayLibrary.Array_Clear` (`self.SplineMeshArray`)))
        (for _index_2 (range (+ (`KismetMathLibrary.SelectInt` (`self.NumberOfRoadSegments`) (- (`self.NumberOfSplinePoints`) 2) (`self.FixedRoadLength`)) 1))
          (bind _output_get (set `self.Index` _index_2))
          (if (`.Visible_15_CEF22AF749349EA8A3D8FA8DE4E55B15` (break `/Game/Core/Engine/SRoadDataStruct` (`|GetArrayItem` (`self.RoadSegments`) _output_get)))
            (bind _returnvalue_12 (`AddComponent|NODE_AddSplineMeshComponent-0`))
            (set `self.SplineMesh` _returnvalue_12)
            (`KismetArrayLibrary.Array_Add` (`self.SplineMeshArray`) (`self.SplineMesh`))
            (`StaticMeshComponent.SetStaticMesh` (`self.SplineMesh`) (`.RoadMesh_2_85382284414C9A30A2F4319C93E8AE63` (break `/Game/Core/Engine/SRoadDataStruct` (`|GetArrayItem` (`self.RoadSegments`) (`self.Index`)))))
            (if (not (`self.EditMode`))
              (for (_array_element _array_index) (`.MaterialOverrides_7_CE0207704C9AC59BFF9241A258D62C8F` (break `/Game/Core/Engine/SRoadDataStruct` (`|GetArrayItem` (`self.RoadSegments`) (`self.Index`))))
                (`/Engine/EditorBlueprintResources/StandardMacros.IsValid` _array_element
                  (:`Is Valid`
                    (`PrimitiveComponent.SetMaterial` (`self.SplineMesh`) _array_index _array_element))))
              (`SceneComponent.K2_AttachToComponent` (`self.SplineMesh`) (`self.DefaultSceneRoot`) "None" "KeepRelative" "KeepRelative" "KeepRelative" true))
            (if (`self.FixedRoadLength`)
              ;[1 1 1] Fixed Length
              (if (!= (`self.Index`) (`self.NumberOfRoadSegments`))
                ;[1 1 1] Define start and end points of mesh
                (`SplineMeshComponent.SetStartAndEnd` (`self.SplineMesh`) _returnvalue_9 (* _returnvalue_10 (`self.TangentLength`)) (`SplineComponent.GetLocationAtDistanceAlongSpline` _spline_3 _returnvalue_11 "Local") (* (`SplineComponent.GetDirectionAtDistanceAlongSpline` _spline_3 _returnvalue_11 "Local") (`self.TangentLength`)) _returnvalue)
                (else
                  (`SplineMeshComponent.SetStartAndEnd` (`self.SplineMesh`) _returnvalue_9 (* _returnvalue_10 (`self.EndTangentLength`)) (`SplineComponent.GetLocationAtSplinePoint` _spline_4 _returnvalue_6 "Local") (* (`SplineComponent.GetDirectionAtSplinePoint` _spline_4 _returnvalue_6 "Local") (`self.EndTangentLength`)) _returnvalue)))
              ;[1 1 1] Set Mesh Scale
              (`SplineMeshComponent.SetStartScale` (`self.SplineMesh`) (`KismetMathLibrary.MakeVector2D` _returnvalue_y_2 _returnvalue_z_2) (not (`self.EditMode`)))
              (`SplineMeshComponent.SetEndScale` (`self.SplineMesh`) (`KismetMathLibrary.MakeVector2D` _returnvalue_y_4 _returnvalue_z_4) (not (`self.EditMode`)))
              ;[1 1 1] Set Roll
              (`SplineMeshComponent.SetStartRoll` (`self.SplineMesh`) (`KismetMathLibrary.DegreesToRadians` (`SplineComponent.GetRollAtDistanceAlongSpline` (`self.Spline`) (* (`self.Index`) (`self.MeshLength`)) "Local")) (not (`self.EditMode`)))
              (`SplineMeshComponent.SetEndRoll` (`self.SplineMesh`) (`KismetMathLibrary.DegreesToRadians` (`SplineComponent.GetRollAtDistanceAlongSpline` _spline (`KismetMathLibrary.SelectFloat` _returnvalue_7 _returnvalue_4 (<= _returnvalue_7 _returnvalue_4)) "Local")) (not (`self.EditMode`)))
              (else
                ;[1 1 1] Point to point
                (if (!= (`self.Index`) (- (`self.NumberOfSplinePoints`) 1))
                  ;[1 1 1] Define start and end points of mesh
                  (`SplineMeshComponent.SetStartAndEnd` (`self.SplineMesh`) _location _tangent _location_3 _tangent_3 _returnvalue_2)
                  (else
                    (`SplineMeshComponent.SetStartAndEnd` (`self.SplineMesh`) _location (0.0 0.0 0.0) _location_2 _tangent_2 _returnvalue_2)))
                ;[1 1 1] Set Mesh Scale
                (`SplineMeshComponent.SetStartScale` (`self.SplineMesh`) (`KismetMathLibrary.MakeVector2D` _returnvalue_y _returnvalue_z) (not (`self.EditMode`)))
                (`SplineMeshComponent.SetEndScale` (`self.SplineMesh`) (`KismetMathLibrary.MakeVector2D` _returnvalue_y_3 _returnvalue_z_3) (not (`self.EditMode`)))
                ;[1 1 1] Set Roll
                (`SplineMeshComponent.SetStartRoll` (`self.SplineMesh`) (`KismetMathLibrary.DegreesToRadians` (`SplineComponent.GetRollAtSplinePoint` (`self.Spline`) (`self.Index`) "Local")) (not (`self.EditMode`)))
                (`SplineMeshComponent.SetEndRoll` (`self.SplineMesh`) (`KismetMathLibrary.DegreesToRadians` (`SplineComponent.GetRollAtSplinePoint` (`self.Spline`) (+ (`self.Index`) 1) "Local")) (not (`self.EditMode`)))))))))
    (elif (not (`self.SplineOnlyMode`))
      (goto _label))))