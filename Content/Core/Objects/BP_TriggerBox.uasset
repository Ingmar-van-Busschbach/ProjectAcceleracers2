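; BP_TriggerBox is a box volume actor sized by two corner variables, with no active event logic of its own.
; Its construction script sets the Box component's world scale to the top-right corner minus the bottom-left.
; It places the Box at the corners' midpoint, rotated by the actor's rotation and offset by its location, so corners act as actor-relative positions.
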(fn `UserConstructionScript`
  (bind _hitboxtoprightcorner (`self.HitboxTopRightCorner`))
  (bind _hitboxbottomleftcorner (`self.HitboxBottomLeftCorner`))
  (bind _box (`self.Box`))
  (`SceneComponent.SetWorldScale3D` _box (- _hitboxtoprightcorner _hitboxbottomleftcorner))
  (`SceneComponent.K2_SetWorldLocation` _box (+ (`KismetMathLibrary.GreaterGreater_VectorRotator` (`KismetMathLibrary.VLerp` _hitboxtoprightcorner _hitboxbottomleftcorner 0.5) (`self.K2_GetActorRotation`)) (`self.K2_GetActorLocation`)) false false))