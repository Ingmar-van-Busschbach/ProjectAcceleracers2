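; Vehicle component that animates a wheel's suspension travel and spin, driven by its parent BP_WheelComponent, which it caches on BeginPlay.
; Each tick it interpolates its world position along the wheel's up axis, following ground distance when grounded or dropping to full arm length when airborne.
; It adds pitch each tick from forward velocity divided by scaled wheel size, without delta-time scaling.
; A wrong parent type or invalid wheel reference prints a debug message.
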(event `self.ReceiveBeginPlay`
  (bind _asbp_wheel_component (cast `/Game/Core/Vehicles/BP_WheelComponent` (`|GetArrayItem` (`self.GetParentComponents`)))
    (:`then`
      (bind _output_get (set `self.WheelRef` _asbp_wheel_component))
      (set `self.RefLocation` (`SceneComponent.RelativeLocation` (`self.GetAttachParent` _output_get))))
    (:`CastFailed`
      (`/Game/Core/Engine/BPFL_DebugFunctions.PrintMessage` "Parent component of animated wheel is not a BP_WheelComponent" "NewEnumerator1"))))

(event `self.ReceiveTick`
  (params (DeltaSeconds :type "Float (single-precision)"))
  (`/Engine/EditorBlueprintResources/StandardMacros.IsValid` (`self.WheelRef`)
    (:`Is Valid`
      (`self.TickSuspension`)
      (`self.TickRotation`))
    (:`Is Not Valid`
      (`/Game/Core/Engine/BPFL_DebugFunctions.PrintMessage` "Wheel reference is not valid" "NewEnumerator1"))))

(event `TickSuspension`
  (bind _wheelref (`self.WheelRef`))
  (bind _returnvalue (`self.K2_GetComponentLocation` _wheelref))
  (bind _returnvalue_2 (`self.GetUpVector` _wheelref))
  (bind (_returnvalue_x _returnvalue_y _returnvalue_z) (`KismetMathLibrary.BreakVector` (`self.K2_GetComponentScale` _wheelref)))
  (bind _suspensionsettings (`/Game/Core/Vehicles/BP_WheelComponent.SuspensionSettings` _wheelref))
  (`self.K2_SetWorldLocation` (`KismetMathLibrary.VInterpTo` (`self.K2_GetComponentLocation`) (`KismetMathLibrary.SelectVector` (- _returnvalue (* _returnvalue_2 (+ (- (`/Game/Core/Vehicles/BP_WheelComponent.GroundDistance` _wheelref) (* _returnvalue_z (`/Game/Core/Vehicles/BP_WheelComponent.WheelSize` _wheelref) 0.5)) (`/Game/Core/Vehicles/PDA_SuspensionSettings.TraceRadius` _suspensionsettings) (`/Game/Core/Vehicles/PDA_SuspensionSettings.TireContactDepth` _suspensionsettings)))) (- _returnvalue (* _returnvalue_2 (`/Game/Core/Vehicles/PDA_SuspensionSettings.ArmLength` _suspensionsettings))) (`/Game/Core/Vehicles/BP_WheelComponent.Grounded` _wheelref)) (`GameplayStatics.GetWorldDeltaSeconds`) 100.0) false true))

(event `TickRotation`
  (bind _wheelref (`self.WheelRef`))
  (bind (_returnvalue_x _returnvalue_y _returnvalue_z) (`KismetMathLibrary.BreakVector` (`self.K2_GetComponentScale` _wheelref)))
  (`self.K2_AddLocalRotation` (`KismetMathLibrary.MakeRotator` 0.0 (* (/ (`KismetMathLibrary.Dot_VectorVector` (`/Game/Core/Vehicles/BP_WheelComponent.LocalVelocity` _wheelref) (`self.GetForwardVector` _wheelref)) (* _returnvalue_z (`/Game/Core/Vehicles/BP_WheelComponent.WheelSize` _wheelref))) -1.0)) false true))