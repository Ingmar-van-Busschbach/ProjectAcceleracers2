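; Wheel component for physics vehicles that applies suspension, grip, drive and steering to the owner's simulating root body.
; Each tick a capsule trace finds the ground and drives an exponential-compression spring-damper force along the hit normal, then lateral grip opposes sideways slip when grounded.
; Acceleration and steering events push at the contact point and yaw the wheel by a speed curve.
; Physical-material grip scales traction; longitudinal grip is defined but never called here.
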(event `self.ReceiveBeginPlay`
  (bind _asprimitive_component (cast `PrimitiveComponent` (`Actor.RootComponent` (`self.GetOwner`)))
    (:`then`
      (if (`self.IsSimulatingPhysics` _asprimitive_component "None")
        (set `self.PhysicsBodyRef` _asprimitive_component)
        (else
          (`/Game/Core/Engine/BPFL_DebugFunctions.PrintMessage` "Owning root component is not physics enabled" "NewEnumerator1"))))
    (:`CastFailed`
      (`/Game/Core/Engine/BPFL_DebugFunctions.PrintMessage` "Owning root component is not physics compatible" "NewEnumerator1"))))

(event `self.ReceiveTick`
  (params (DeltaSeconds :type "Float (single-precision)"))
  (`/Engine/EditorBlueprintResources/StandardMacros.IsValid` (`self.PhysicsBodyRef`)
    (:`Is Valid`
      (`|ExecutionSequence`
        (:`then_0`
          (`self.TickSuspension`))
        (:`then_1`
          (if (`self.Grounded`)
            (bind _velocity (`self.GetLocalLinearVelocity`))
            (set `self.LocalVelocity` _velocity)
            (`|ExecutionSequence`
              (:`then_0`
                (`self.TickLateralGrip`)))))))
    (:`Is Not Valid`
      (`/Game/Core/Engine/BPFL_DebugFunctions.PrintMessage` "Physics body reference is not valid." "NewEnumerator1" true))))

(event `TickSuspension`
  (bind _returnvalue (`self.K2_GetComponentLocation`))
  (bind (_returnvalue_x _returnvalue_y _returnvalue_z) (`KismetMathLibrary.BreakVector` (`self.K2_GetComponentScale`)))
  (bind _traceradius (`/Game/Core/Vehicles/PDA_SuspensionSettings.TraceRadius` (`self.SuspensionSettings`)))
  (bind (_outhit _returnvalue_2) (`KismetSystemLibrary.CapsuleTraceSingle` _returnvalue (- (- _returnvalue (* (`self.GetUpVector`) (* _returnvalue_z (`self.WheelSize`) 0.5))) (* (`self.GetUpVector` (`self.PhysicsBodyRef`)) (* (`/Game/Core/Vehicles/PDA_SuspensionSettings.ArmLength` (`self.SuspensionSettings`)) (`self.SuspensionLengthModifier`)))) _traceradius _traceradius "TraceTypeQuery1" false (`|MakeArray` (`self.GetOwner`)) (select `bool` (`/Game/Core/Engine/BPFL_GlobalConstants.GlobalDebug`) :`true` "ForOneFrame" :!type "EDrawDebugTrace Enum")))
  (bind _output_get (set `self.Grounded` _returnvalue_2))
  (`/Game/Core/Engine/BPFL_DebugFunctions.PrintMessage` (`KismetStringLibrary.Concat_StrStr` (`KismetSystemLibrary.GetObjectName` self) ": Grounded: " (`KismetStringLibrary.Conv_BoolToString` _output_get) " | On surface: " (`KismetSystemLibrary.GetObjectName` (`self.GroundSurface`))) "NewEnumerator0" true)
  (if _output_get
    (`self.SetHitData` _outhit)
    (bind (_suspensionforce _suspensioncompression) (`self.CalculateSuspensionForce` _outhit))
    (set `self.SuspensionForce` _suspensionforce)
    (set `self.SuspensionCompressionLastFrame` _suspensioncompression)
    (`PrimitiveComponent.AddForceAtLocation` (`self.PhysicsBodyRef`) (* (`self.GroundNormal`) (`self.SuspensionForce`)) (`self.K2_GetComponentLocation`) "None")))

(event `TickLateralGrip`
  (bind _physicsbodyref (`self.PhysicsBodyRef`))
  (bind _gripsettings (`self.GripSettings`))
  (bind (_value _returnvalue) (`BlueprintMapLibrary.Map_Find` (`/Game/Core/Vehicles/PDA_GripSettings.SurfaceGripMap` _gripsettings) (`self.GroundSurface`)))
  (bind (_returnvalue_lateralgrip _returnvalue_lateralfriction) (break `/Game/Core/Engine/SGripStruct` (select `bool` _returnvalue :`false` (`/Game/Core/Vehicles/PDA_GripSettings.StandardGrip` _gripsettings) :`true` _value)))
  (bind _returnvalue_2 (`PrimitiveComponent.GetPhysicsLinearVelocityAtPoint` (`self.PhysicsBodyRef`) (`self.K2_GetComponentLocation`) "None"))
  (bind _returnvalue_3 (`KismetMathLibrary.Dot_VectorVector` _returnvalue_2 (`self.GetRightVector`)))
  (`PrimitiveComponent.AddForceAtLocation` _physicsbodyref (* (`self.GetRightVector` _physicsbodyref) (+ (* _returnvalue_3 -1.0 _returnvalue_lateralgrip) (* (`KismetMathLibrary.SignOfFloat` _returnvalue_3) -1.0 _returnvalue_lateralfriction))) (`self.K2_GetComponentLocation`) "None"))

(event `TickLongitunalGrip`
  (bind _physicsbodyref (`self.PhysicsBodyRef`))
  (bind _gripsettings (`self.GripSettings`))
  (bind (_value _returnvalue) (`BlueprintMapLibrary.Map_Find` (`/Game/Core/Vehicles/PDA_GripSettings.SurfaceGripMap` _gripsettings) (`self.GroundSurface`)))
  (bind (_returnvalue_lateralgrip _returnvalue_lateralfriction _returnvalue_longitunalfriction) (break `/Game/Core/Engine/SGripStruct` (select `bool` _returnvalue :`false` (`/Game/Core/Vehicles/PDA_GripSettings.StandardGrip` _gripsettings) :`true` _value)))
  (bind _returnvalue_2 (`PrimitiveComponent.GetPhysicsLinearVelocityAtPoint` (`self.PhysicsBodyRef`) (`self.K2_GetComponentLocation`) "None"))
  (`PrimitiveComponent.AddForceAtLocation` _physicsbodyref (* (`self.GetForwardVector` _physicsbodyref) (* (`KismetMathLibrary.SignOfFloat` (`KismetMathLibrary.Dot_VectorVector` _returnvalue_2 (`self.GetForwardVector`))) -1.0 _returnvalue_longitunalfriction)) (`self.K2_GetComponentLocation`) "None"))

(event `TickAcceleration`
  (params (Force :type "Float (double-precision)"))
  (bind _physicsbodyref (`self.PhysicsBodyRef`))
  (if (`self.Grounded`)
    (`PrimitiveComponent.AddForceAtLocation` _physicsbodyref (* (`self.GetForwardVector` _physicsbodyref) (* Force (`self.GetAccelerationModifier`))) (`self.GroundLocation`) "None")))

(event `TickSteering`
  (params (Input :type "Float (double-precision)"))
  (bind _relativerotation (`self.RelativeRotation`))
  (bind _steeringsettings (`self.SteeringSettings`))
  (`self.K2_SetRelativeRotation` (`KismetMathLibrary.RInterpTo_Constant` _relativerotation (`KismetMathLibrary.MakeRotator` 0.0 0.0 (* Input (`KismetMathLibrary.GetRuntimeFloatCurveValue` (`/Game/Core/Vehicles/PDA_SteeringSettings.SteeringRateOverSpeed` _steeringsettings) (/ (`KismetMathLibrary.Dot_VectorVector` (`self.LocalVelocity`) (`self.GetForwardVector` (`self.PhysicsBodyRef`))) (`/Game/Core/Vehicles/PDA_SteeringSettings.SteeringMaxSpeed` _steeringsettings)) 1.0) (`/Game/Core/Vehicles/PDA_SteeringSettings.SteeringMaxAngle` _steeringsettings))) (`GameplayStatics.GetWorldDeltaSeconds`) (`KismetMathLibrary.SelectFloat` (`/Game/Core/Vehicles/PDA_SteeringSettings.SteeringRate` _steeringsettings) (`/Game/Core/Vehicles/PDA_SteeringSettings.SteeringRateNeutral` _steeringsettings) (> (`KismetMathLibrary.SignOfFloat` (* Input (.yaw _relativerotation))) 0.0))) false true))

(fn `CalculateSuspensionForce`
  (params (`Hit Result` :type "HitResult Structure"))
  (returns (SuspensionForce :type "Float (double-precision)") (SuspensionCompression :type "Float (double-precision)"))
  (bind (_returnvalue_x _returnvalue_y _returnvalue_z) (`KismetMathLibrary.BreakVector` (`self.K2_GetComponentScale`)))
  (bind _suspensionsettings (`self.SuspensionSettings`))
  (bind _armlength (`/Game/Core/Vehicles/PDA_SuspensionSettings.ArmLength` (`self.SuspensionSettings`)))
  (bind _returnvalue (`KismetMathLibrary.MultiplyMultiply_FloatFloat` (/ (- _armlength (`KismetMathLibrary.FClamp` (- (`.Distance` (`GameplayStatics.BreakHitResult` `Hit Result`)) (* _returnvalue_z (`self.WheelSize`) 0.5)) 0.0 _armlength)) _armlength) (`/Game/Core/Vehicles/PDA_SuspensionSettings.CompressionExponent` _suspensionsettings)))
  (return (+ (* (/ (- _returnvalue (`self.SuspensionCompressionLastFrame`)) (`GameplayStatics.GetWorldDeltaSeconds`)) (* (`/Game/Core/Vehicles/PDA_SuspensionSettings.Damping` (`self.SuspensionSettings`)) (`/Game/Core/Engine/BPFL_GlobalConstants.GlobalGravity`))) (* _returnvalue (* (`/Game/Core/Vehicles/PDA_SuspensionSettings.Stiffness` _suspensionsettings) (`/Game/Core/Engine/BPFL_GlobalConstants.GlobalGravity`)))) _returnvalue))

(fn `GetAccelerationModifier`
  (returns (AccelerationModifier :type "Float (double-precision)"))
  (bind _gripsettings (`self.GripSettings`))
  (bind (_value _returnvalue) (`BlueprintMapLibrary.Map_Find` (`/Game/Core/Vehicles/PDA_GripSettings.SurfaceGripMap` _gripsettings) (`self.GroundSurface`)))
  (bind (_returnvalue_lateralgrip _returnvalue_lateralfriction _returnvalue_longitunalfriction _returnvalue_accelerationmodifier) (break `/Game/Core/Engine/SGripStruct` (select `bool` _returnvalue :`false` (`/Game/Core/Vehicles/PDA_GripSettings.StandardGrip` _gripsettings) :`true` _value)))
  (return _returnvalue_accelerationmodifier))

(fn `GetLateralFriction`
  (returns (LateralFriction :type "Float (double-precision)"))
  (bind _gripsettings (`self.GripSettings`))
  (bind (_value _returnvalue) (`BlueprintMapLibrary.Map_Find` (`/Game/Core/Vehicles/PDA_GripSettings.SurfaceGripMap` _gripsettings) (`self.GroundSurface`)))
  (bind (_returnvalue_lateralgrip _returnvalue_lateralfriction) (break `/Game/Core/Engine/SGripStruct` (select `bool` _returnvalue :`false` (`/Game/Core/Vehicles/PDA_GripSettings.StandardGrip` _gripsettings) :`true` _value)))
  (return _returnvalue_lateralfriction))

(fn `GetLateralGrip`
  (returns (LateralGrip :type "Float (double-precision)"))
  (bind _gripsettings (`self.GripSettings`))
  (bind (_value _returnvalue) (`BlueprintMapLibrary.Map_Find` (`/Game/Core/Vehicles/PDA_GripSettings.SurfaceGripMap` _gripsettings) (`self.GroundSurface`)))
  (bind _returnvalue_lateralgrip (break `/Game/Core/Engine/SGripStruct` (select `bool` _returnvalue :`false` (`/Game/Core/Vehicles/PDA_GripSettings.StandardGrip` _gripsettings) :`true` _value)))
  (return _returnvalue_lateralgrip))

(fn `GetLocalLinearVelocity`
  (returns (Velocity :type "Vector Structure"))
  (bind _returnvalue (`PrimitiveComponent.GetPhysicsLinearVelocityAtPoint` (`self.PhysicsBodyRef`) (`self.GroundLocation`) "None"))
  (return _returnvalue))

(fn `SetHitData`
  (params (HitResult :type "HitResult Structure"))
  (bind (_bblockinghit _binitialoverlap _time _distance _location _impactpoint _normal _impactnormal _physmat) (`GameplayStatics.BreakHitResult` HitResult))
  (set `self.GroundDistance` _distance)
  (set `self.GroundLocation` _impactpoint)
  (set `self.GroundSurface` _physmat)
  (set `self.GroundNormal` _impactnormal))